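; Moving platform actor that carries its mesh along a spline path, starting automatically on BeginPlay.
; A timeline, with play rate set from the Rate variable, outputs a normalized distance that is scaled by spline length and sampled as a world location.
; Only the mesh's location is updated, without sweep or rotation.
; The construction script applies the configurable static mesh and material.
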(event `Platform start`
  (bind (_direction _spline_distance) (`Timeline|Motion Timeline` :!via `PlayFromStart`)
    (:`Update`
      (`SceneComponent.K2_SetWorldLocation` (`self.Platform Mesh`) (`SplineComponent.GetLocationAtDistanceAlongSpline` (`self.Spline`) (* _spline_distance (`SplineComponent.GetSplineLength` (`self.Spline`))) "World") false false))))

(event `self.ReceiveBeginPlay`
  (`TimelineComponent.SetPlayRate` (`self.Motion Timeline`) (`self.Rate`))
  (`self.Platform start`))

(fn `UserConstructionScript`
  (bind _platform_mesh (`self.Platform Mesh`))
  (`StaticMeshComponent.SetStaticMesh` _platform_mesh (`self.StaticMesh`))
  (`PrimitiveComponent.SetMaterial` _platform_mesh 0 (`self.Material`)))