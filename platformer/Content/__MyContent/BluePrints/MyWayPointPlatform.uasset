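; Moving platform actor that travels along an array of waypoint actors, with configurable mesh, material, speed rate and optional looping.
; BeginPlay hides the waypoints and calls PlatformStart inside that loop, while Start and Stop functions expose control.
; A timeline lerps the platform between the current and next waypoint positions.
; Its event track advances the indices and replays, or with Loop jumps back to the first waypoint at path end.
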(event `PlatformStart`
  (bind _motion_timeline (`self.Motion Timeline`))
  (`self.setFirst Waypoint`)
  (`TimelineComponent.SetPlayRate` _motion_timeline (`self.SpeedRate`))
  (`TimelineComponent.PlayFromStart` _motion_timeline))

(event `self.ReceiveBeginPlay`
  (for _array_element (`self.WayPoints`)
    (`self.SetActorHiddenInGame` _array_element true)
    (`self.PlatformStart`)))

(fn `Path is Finished`
  (returns (IsFinished :type Boolean))
  (return (== (`self.Next Waypoint index`) (- (`KismetArrayLibrary.Array_Length` (`self.WayPoints`)) 1))))

(fn `setFirst Waypoint`
  (set `self.Current Waypoint index` 0)
  (set `self.Next Waypoint index` 1)
  (`self.SetPositions`))

(fn `SetNextWaypoint`
  (bind _result (`/Engine/EditorBlueprintResources/StandardMacros.IncrementInt` (`self.Current Waypoint index`))
    (:`  `
      (set `self.Next Waypoint index` (+ _result 1))
      (`self.SetPositions`))))

(fn `SetPositions`
  (bind _waypoints (`self.WayPoints`))
  (set `self.Current WayPoint Postion ` (`self.K2_GetActorLocation` (`|GetArrayItem` _waypoints (`self.Current Waypoint index`))))
  (set `self.Next WayPoint Position` (`self.K2_GetActorLocation` (`|GetArrayItem` _waypoints (`self.Next Waypoint index`)))))

(fn `start`
  (`self.PlatformStart`))

(fn `Stop`
  (`TimelineComponent.Stop` (`self.Motion Timeline`)))

(fn `UserConstructionScript`
  (bind _platformmesh (`self.PlatformMesh`))
  (`StaticMeshComponent.SetStaticMesh` _platformmesh (`self.StaticMesh`))
  (`PrimitiveComponent.SetMaterial` _platformmesh 0 (`self.Material`)))